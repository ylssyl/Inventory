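; Interactive door actor that shows a text prompt on Enter, hides it on Exit, and swings open or closed when used.
; StartInteractive picks the swing direction from the world X sign of the direction to the user, then plays or reverses the DoorAnimation timeline to yaw SMDoor up to 90 degrees.
; When the timeline finishes it updates IsOpen and ends the interaction, which makes the Box ignore or block Pawns.
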(event EventBeginPlay
  (Rendering|SetVisibility (Variables|Default|GetTextRender) false false))

(event Collision|EventActorBeginOverlap
  (params (OtherActor :type Actor%20Object%20Reference)))

(event EventTick
  (params (DeltaSeconds :type Float%20%28single-precision%29)))

(event EventEnter
  (params (User :type Actor%20Object%20Reference))
  (Rendering|SetVisibility (Variables|Default|GetTextRender) true false))

(event EventStayTick
  (params (User :type Actor%20Object%20Reference) (DeletaTime :type Float%20%28single-precision%29)))

(event EventExit
  (params (User :type Actor%20Object%20Reference))
  (Rendering|SetVisibility (Variables|Default|GetTextRender) false false))

(event EventStartInteractive
  (params (User :type Actor%20Object%20Reference) (InteractiveComponent :type Interactive%20Component%20Object%20Reference))
  (bind _dooranimation (Variables|Default|GetDoorAnimation))
  (Variables|Default|SetInteractive%20Component InteractiveComponent)
  (if (> (.x (Math|Vector|GetUnitDirection(Vector) (Transformation|GetActorLocation) (Transformation|GetActorLocation User))) 0.0)
    (Variables|Default|SetOpenDir -1.0)
    (else
      (Variables|Default|SetOpenDir 1.0)))
  (if (Variables|Default|GetIsOpen)
    (Utilities|String|Reverse _dooranimation)
    (else
      (Audio|Components|Audio|Play _dooranimation))))

(event EventInteractiveTick
  (params (User :type Actor%20Object%20Reference) (DeletaTime :type Float%20%28single-precision%29) (InteractiveComponent :type Interactive%20Component%20Object%20Reference)))

(event EventEndInteractive
  (params (User :type Actor%20Object%20Reference))
  (if (Variables|Default|GetIsOpen)
    (Collision|SetCollisionResponsetoChannel (Variables|Default|GetBox) "ECC_Pawn" "ECR_Ignore")
    (else
      (Collision|SetCollisionResponsetoChannel (Variables|Default|GetBox) "ECC_Pawn" "ECR_Block"))))

(fn ConstructionScript)