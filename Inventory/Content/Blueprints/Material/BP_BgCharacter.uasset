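; Modular character actor that mirrors the player BP_Character's equipped gear on separate hat, jacket, gloves, pants and boots meshes.
; The construction script binds all five meshes to the base skeletal mesh with master pose.
; On BeginPlay it subscribes to the player's equip and clear notifications.
; Equipping looks up the item Id in a DataTable to set that part's mesh, while clearing matches EquipmentPart against grid-slot rows to empty it.
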(event Custom|TryToClear
  (CallFunction|ClearSkeletalMesh))

(event Custom|TryToEquip
  (CallFunction|Equipment))

(event EventBeginPlay
  (bind _ascharacter_bp (Utilities|Casting|CastToBP_Character (Game|Player|GetPlayerPawn 0)))
  (Variables|Default|SetAs%20Character%20BP _ascharacter_bp)
  (EventDispatchers|BindEventtoNoticeUpdateEquipment _ascharacter_bp (delegate Custom|TryToEquip))
  (EventDispatchers|BindEventtoNoticeClearEquipItem (Variables|Default|GetAs%20Character%20BP) (delegate Custom|TryToClear)))

(event Collision|EventActorBeginOverlap
  (params (OtherActor :type Actor%20Object%20Reference)))

(event EventTick
  (params (DeltaSeconds :type Float%20%28single-precision%29)))

(fn ConstructionScript
  (CallFunction|SetMasterPose))

(fn Equipment
  (bind _returnvalue (Utilities|GetDataTableRow "/Game/DataTable/EquipmentItemAttr_DT.EquipmentItemAttr_DT" (Utilities|String|StringToName (Utilities|String|ToString(Integer) (Variables|/Game/Blueprints/GamePlay/BP_Character.BP_Character_C|GetId (Variables|Default|GetAs%20Character%20BP)))))
    (:then
      (switch name (.Part (Utilities|Struct|BreakEquipmentItemAttr_ST _returnvalue))
        (:Hat
          (Class|SkinnedMeshComponent|SetSkeletalMesh (Variables|Default|GetHat) (.EquipmentSkeletalMesh (Utilities|Struct|BreakEquipmentItemAttr_ST _returnvalue)) true))
        (:Jaket
          (Class|SkinnedMeshComponent|SetSkeletalMesh (Variables|Default|GetJaket) (.EquipmentSkeletalMesh (Utilities|Struct|BreakEquipmentItemAttr_ST _returnvalue)) true))
        (:Gloves
          (Class|SkinnedMeshComponent|SetSkeletalMesh (Variables|Default|GetGloves) (.EquipmentSkeletalMesh (Utilities|Struct|BreakEquipmentItemAttr_ST _returnvalue)) true))
        (:Pants
          (Class|SkinnedMeshComponent|SetSkeletalMesh (Variables|Default|GetPants) (.EquipmentSkeletalMesh (Utilities|Struct|BreakEquipmentItemAttr_ST _returnvalue)) true))
        (:Boots
          (Class|SkinnedMeshComponent|SetSkeletalMesh (Variables|Default|GetBoots) (.EquipmentSkeletalMesh (Utilities|Struct|BreakEquipmentItemAttr_ST _returnvalue)) true))))))

(fn SetMasterPose
  (Class|SkinnedMeshComponent|SetMasterPoseComponent (Variables|Default|GetHat) (Variables|Default|GetSkeletalMesh) false))

(fn ClearSkeletalMesh
  (bind _index (Utilities|FlowControl|ForLoopwithBreak 0 5)
    (:LoopBody
      (bind _output_get (Variables|Default|SetIndex _index))
      (bind _returnvalue (Utilities|GetDataTableRow "/Game/DataTable/EquipmentGridType1Attr_DT.EquipmentGridType1Attr_DT" (Utilities|String|StringToName (Utilities|String|ToString(Integer) _output_get)))
        (:then
          (if (Utilities|Name|Equal(Name) (.EquipmentGridPart (Utilities|Struct|BreakEquipmentGridType1Attr _returnvalue)) (Variables|/Game/Blueprints/GamePlay/BP_Character.BP_Character_C|GetEquipment%20Part (Variables|Default|GetAs%20Character%20BP)))
            (if (== (Variables|Default|GetIndex) 0)
              (Class|SkinnedMeshComponent|SetSkeletalMesh (Variables|Default|GetHat) 0 true)
              (elif (== (Variables|Default|GetIndex) 1)
                (Class|SkinnedMeshComponent|SetSkeletalMesh (Variables|Default|GetJaket) 0 true)
                (elif (== (Variables|Default|GetIndex) 2)
                  (Class|SkinnedMeshComponent|SetSkeletalMesh (Variables|Default|GetGloves) 0 true)
                  (elif (== (Variables|Default|GetIndex) 4)
                    (Class|SkinnedMeshComponent|SetSkeletalMesh (Variables|Default|GetPants) 0 true)
                    (elif (== (Variables|Default|GetIndex) 5)
                      (Class|SkinnedMeshComponent|SetSkeletalMesh (Variables|Default|GetBoots) 0 true))))))))))))