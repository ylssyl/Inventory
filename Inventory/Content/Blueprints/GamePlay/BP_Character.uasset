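; Player character Blueprint for sword melee combat, with interaction, bag and equipment UI toggles, and mouse cursor toggling.
; Equipment sync shows or hides the sword and scabbard, and toggling combat re-sockets them and switches rotation mode.
; Attacks activate a GAS ability; attack ticks sphere-trace sword and feet, sending a damage gameplay event once per new actor.
; Directional roll montages move the character through animation curves while disabling damage.
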(event OnComponentHit(CapsuleComponent)
  (params (HitComponent :type Primitive%20Component%20Object%20Reference) (OtherActor :type Actor%20Object%20Reference) (OtherComp :type Primitive%20Component%20Object%20Reference) (NormalImpulse :type Vector :default "0, 0, 0") (Hit :type Hit%20Result%20Structure%20%28by%20ref%29)))

(event EventBeginPlay
  (bind _aspc_bp (Utilities|Casting|CastToPC_BP (Pawn|GetController)))
  (Variables|Default|SetAs%20PC%20BP _aspc_bp)
  (Class|InventoryCharacterBase|GiveAbility))

(event Collision|EventActorBeginOverlap
  (params (OtherActor :type Actor%20Object%20Reference)))

(event EventTick
  (params (DeltaSeconds :type Float%20%28single-precision%29))
  (bind _returnvalue (Transformation|GetVelocity))
  (bind _movementdirection (Variables|Default|GetMovementDirection))
  (bind _returnvalue_2 (Math|Vector|ProjectVectorontoPlane _returnvalue "0,0.000000,1.000000"))
  (Transformation|SetWorldRotation (Variables|Default|GetCharacterDirection) (Transformation|GetActorRotation) false false)
  (Transformation|SetWorldRotation _movementdirection (Math|Conversions|RotationFromXVector _returnvalue_2) false false)
  (Rendering|SetVisibility _movementdirection (not (Math|Float|NearlyEqual(Float) (Math|Vector|VectorLength _returnvalue_2) 0.0 1e-06)) false))

(event Input|KeyboardEvents|E
  (params (Key :type Key%20Structure :default "None"))
  (:Pressed
    (Class|InventoryCharacterBase|UseShortcutsItem)))

(event Input|KeyboardEvents|F
  (params (Key :type Key%20Structure))
  (:Pressed
    (Class|InteractiveComponent|StartInteractive (Variables|Default|GetInteractiveComponent))))

(event Input|ActionEvents|InputActionShowMouse
  (params (Key :type Key%20Structure))
  (:Pressed
    (CallFunction|ShowMouse)))

(event Input|AxisEvents|InputAxisTurn
  (params (AxisValue :type Float%20%28single-precision%29))
  (Pawn|Input|AddControllerYawInput AxisValue))

(event Input|AxisEvents|InputAxisLookUp
  (params (AxisValue :type Float%20%28single-precision%29))
  (Pawn|Input|AddControllerPitchInput AxisValue))

(event EventSyncEquipment
  (params (InId :type Integer))
  (Variables|Default|SetId InId)
  (Default|CallNoticeUpdateEquipment))

(event EventSyncClearEquipment
  (params (InEquipmentPart :type Name :default "None"))
  (Variables|Default|SetEquipment%20Part InEquipmentPart)
  (Default|CallNoticeClearEquipItem))

(event EventSyncWeapon
  (params (InId :type Integer))
  (Variables|Default|SetWeaponId InId)
  (CallFunction|ShowCovered))

(event EventSyncClearWeapon
  (CallFunction|SetCovered))

(event Input|ActionEvents|InputActionToggleBagWidget
  (params (Key :type Key%20Structure))
  (:Pressed
    (Class|BPIToggleBagWidget|ToggleBagWidget(Message) (HUD|GetHUD (Variables|Default|GetAs%20PC%20BP)))))

(event Input|ActionEvents|InputActionToggleEquipmentWidget
  (params (Key :type Key%20Structure))
  (:Pressed
    (Class|BPIToggleBagWidget|ToggleEquipWidget(Message) (HUD|GetHUD (Variables|Default|GetAs%20PC%20BP)))))

(event Custom|TryToggleWeapon
  (params (IsEquip :type Boolean))
  (Utilities|FlowControl|Sequence
    (:then_0
      (bind _output_get (Variables|/Script/Engine.CharacterMovementComponent|SetbUseControllerDesiredRotation (Variables|Character|GetCharacterMovement) (not (Variables|Default|GetIsCombat))))
      (Variables|/Script/Engine.CharacterMovementComponent|SetbOrientRotationToMovement (Variables|Character|GetCharacterMovement) (not _output_get)))
    (:then_1
      (if (not (Variables|Default|GetIsCombat))
        (Variables|Default|SetHandWeapon (Variables|Default|GetSM_Sword))
        (else
          (Variables|Default|SetHandWeapon 0))))
    (:then_2
      (Transformation|AttachComponentToComponent (Variables|Default|GetSM_Sword) (Variables|Character|GetMesh) (select (not (Variables|Default|GetIsCombat)) "hand_rSocket" "SwordSocket") "SnapToTarget" "SnapToTarget" "SnapToTarget" true)
      (Transformation|AttachComponentToComponent (Variables|Default|GetSM_cover) (Variables|Character|GetMesh) (select (not (Variables|Default|GetIsCombat)) "hand_lSocket" "ScabbardSocket") "SnapToTarget" "SnapToTarget" "SnapToTarget" true))
    (:then_3
      (Utilities|FlowControl|FlipFlop
        (:A
          (Variables|Default|SetIsCombat true))
        (:B
          (Variables|Default|SetIsCombat false))))))

(event Input|ActionEvents|InputActionswitchover
  (params (Key :type Key%20Structure :default "None"))
  (:Pressed
    (if (CallFunction|CanbeToggleWeapon)
      (CallFunction|TryToggleWeapon (CallFunction|GetEquip)))))

(event Custom|TryAttack
  (if (CallFunction|GetAttack)
    (Abilities|TryActivateAbilitybyClass (Variables|Default|GetAbilitySystemComponent) "/Game/Blueprints/GameplayAbility/GA_MeleeAttack.GA_MeleeAttack_C" true)))

(event Custom|OnBeginAttack
  (Variables|Default|SetCurrentAttackCombo (Math|Integer|%(Integer) (+ (Variables|Default|GetCurrentAttackCombo) 1) (Utilities|Array|Length (Variables|Default|GetAttackComboSections)))))

(event Custom|OnAttackTick
  (params (DamageSection :type Name) (AttackLocation :type Vector))
  (bind (_damagearray _successed) (CallFunction|BodyFootrDamageTrace))
  (bind (_damagearray_2 _successed_2) (CallFunction|SwordDamageTrace))
  (Variables|Default|SetDamage%20Section DamageSection)
  (Variables|Default|SetAttack%20Location AttackLocation)
  (Utilities|FlowControl|Sequence
    (:then_0
      (if _successed_2
        (for _array_element _damagearray_2
          (bind _returnvalue (Utilities|Array|AddUnique (Variables|Default|GetDamageArray) _array_element))
          (if (not (< _returnvalue 0))
            (Ability|SendGameplayEventtoActor self "(TagName=\"skill.melee.dealDamage\")" (Utilities|Struct|MakeGameplayEventData "(TagName=\"skill.melee.dealDamage\")" 0 _array_element 0 0 "()" "(GameplayTags=)" "(GameplayTags=((TagName=\"skill.melee.dealDamage\")))"))))))
    (:then_1
      (if _successed
        (for _array_element_2 _damagearray
          (bind _returnvalue_2 (Utilities|Array|AddUnique (Variables|Default|GetDamageArray) 0))
          (if (not (< _returnvalue_2 0))
            (Ability|SendGameplayEventtoActor self "(TagName=\"skill.melee.dealDamage\")" (Utilities|Struct|MakeGameplayEventData "(TagName=\"skill.melee.dealDamage\")" _array_element_2 0 0 0 "()" "(GameplayTags=)" "(GameplayTags=((TagName=\"skill.melee.dealDamage\")))"))))))
    (:then_2
      (if true
        (for _array_element_3 (.DamageArray (CallFunction|BodyFootlDamageTrace))
          (bind _returnvalue_3 (Utilities|Array|AddUnique (Variables|Default|GetDamageArray) 0))
          (if (not (< _returnvalue_3 0))
            (Ability|SendGameplayEventtoActor self "(TagName=\"skill.melee.dealDamage\")" (Utilities|Struct|MakeGameplayEventData "(TagName=\"skill.melee.dealDamage\")" 0 0 0 0 "()" "(GameplayTags=)" "(GameplayTags=((TagName=\"skill.melee.dealDamage\")))"))))))))

(event Custom|OnAttack
  (params (DamageSection :type Name) (AttackLocation :type Vector)))

(event Custom|OnEndAttack
  (Utilities|Array|Clear (Variables|Default|GetDamageArray)))

(event Input|ActionEvents|InputActionAttack
  (params (Key :type Key%20Structure :default "None"))
  (:Pressed
    (CallFunction|TryAttack)))

(event Custom|TryTakeDamage
  (params (DamageSection :type Name) (AttackerLocation :type Vector))
  (if (CallFunction|CanTakeDamage)
    (Variables|Default|SetAttackerLocation AttackerLocation)
    (Animation|Montage|PlayMontage (Variables|Character|GetMesh) "/Game/Blueprints/Animation/Damage/AM_DamageAnim.AM_DamageAnim" 1.0 0.0 (Utilities|Name|MakeLiteralName "B"))))

(event Game|Damage|EventAnyDamage
  (params (Damage :type Float%20%28single-precision%29) (DamageType :type Damage%20Type%20Object%20Reference) (InstigatedBy :type Controller%20Object%20Reference) (DamageCauser :type Actor%20Object%20Reference))
  (Development|PrintString (Utilities|String|ToString(Boolean) (.bSuccess (Utilities|Casting|CastToCharacter_BP DamageCauser))))
  (CallFunction|TryTakeDamage "None" "0, 0, 0"))

(event Custom|OnEndRoll
  (bind _charactermovement (Variables|Character|GetCharacterMovement))
  (Variables|Default|SetbCanBeDamaged true)
  (Variables|/Script/Engine.CharacterMovementComponent|SetbUseControllerDesiredRotation _charactermovement true)
  (Variables|/Script/Engine.CharacterMovementComponent|SetbOrientRotationToMovement _charactermovement false)
  (Pawn|Components|CharacterMovement|SetMovementMode _charactermovement "MOVE_Walking" 0))

(event Custom|TryRoll
  (if (CallFunction|CanRoll)
    (Animation|Montage|PlayMontage (Variables|Character|GetMesh) "/Game/Blueprints/Animation/Roll/AM_RollAnim.AM_RollAnim" 1.0 0.0 (CallFunction|GetRollSection)
      (:then
        (Variables|Default|SetIsRoll true))
      (:OnInterrupted
        (CallFunction|OnEndRoll)))))

(event Custom|OnBeginRoll
  (bind _charactermovement (Variables|Character|GetCharacterMovement))
  (Variables|Default|SetbCanBeDamaged false)
  (Variables|/Script/Engine.CharacterMovementComponent|SetbUseControllerDesiredRotation _charactermovement false)
  (Variables|/Script/Engine.CharacterMovementComponent|SetbOrientRotationToMovement _charactermovement true)
  (Pawn|Components|CharacterMovement|SetMovementMode _charactermovement "MOVE_None" 0))

(event Custom|OnRollTick
  (params (DeltaTime :type Float%20%28single-precision%29))
  (bind _returnvalue (Math|Float|MakeLiteralFloat 3e+01))
  (bind _mesh (Variables|Character|GetMesh))
  (bind _returnvalue_2 (Components|SkeletalMesh|GetAnimInstance _mesh))
  (bind _returnvalue_3 (* DeltaTime _returnvalue))
  (bind _returnvalue_4 (Animation|Curves|GetCurveValue _returnvalue_2 "RollOffsetX"))
  (bind _returnvalue_5 (Animation|Curves|GetCurveValue _returnvalue_2 "RollOffsetY"))
  (bind _returnvalue_6 (* _returnvalue_4 -1.0))
  (bind _returnvalue_7 (Math|Vector|MakeVector _returnvalue_5 _returnvalue_6 0.0))
  (bind _returnvalue_8 (* _returnvalue_7 _returnvalue_3))
  (bind _returnvalue_9 (* _returnvalue_8 2.0))
  (Development|PrintString (Utilities|String|ToString(Vector) _returnvalue_9) true true "(R=0.000000,G=0.660000,B=1.000000,A=1.000000)" 0.0)
  (Transformation|AddActorLocalOffset _returnvalue_9 true false))

(event Input|ActionEvents|InputActionRoll
  (params (Key :type Key%20Structure :default "None"))
  (:Pressed
    (CallFunction|TryRoll)))

(fn ConstructionScript)

(fn GetCameraRotation
  (return (Camera|GetCameraRotation (Game|GetPlayerCameraManager 0))))

(fn ShowMouse
  (bind _as_pc_bp (Variables|Default|GetAs%20PC%20BP))
  (if (not (Variables|/Script/Engine.PlayerController|GetbShowMouseCursor (Variables|Default|GetAs%20PC%20BP)))
    (Input|SetInputModeGameandUI (Variables|Default|GetAs%20PC%20BP) 0 "LockAlways" true)
    (Variables|/Script/Engine.PlayerController|SetbShowMouseCursor (Variables|Default|GetAs%20PC%20BP) true)
    (else
      (Input|SetInputModeGameOnly _as_pc_bp)
      (Variables|/Script/Engine.PlayerController|SetbShowMouseCursor _as_pc_bp false))))

(fn GetIsJump
  (return (not (Variables|Default|GetIsJump))))

(fn GetIsArmed
  (return (and (Utilities|IsValid (Variables|Default|GetHandWeapon)) (!= (Variables|Default|GetWeaponId) 0))))

(fn GetEquip
  (return (Math|Boolean|ANDBoolean (or (Utilities|Enum|Equal(Enum) (Variables|Default|GetEquipState) "NewEnumerator0") (Utilities|Enum|Equal(Enum) (Variables|Default|GetEquipState) "NewEnumerator2")) (not (CallFunction|GetIsArmed)) (Variables|Default|GetIsCombat))))

(fn GetUnEquip
  (return (and (or (Utilities|Enum|Equal(Enum) (Variables|Default|GetEquipState) "NewEnumerator1") (Utilities|Enum|Equal(Enum) (Variables|Default|GetEquipState) "NewEnumerator0")) (CallFunction|GetIsArmed))))

(fn SetCovered
  (Development|SetHiddeninGame (Variables|Default|GetSM_cover) true false)
  (Development|SetHiddeninGame (Variables|Default|GetSM_Sword) true false))

(fn ShowCovered
  (Development|SetHiddeninGame (Variables|Default|GetSM_cover) false false)
  (Development|SetHiddeninGame (Variables|Default|GetSM_Sword) false false))

(fn CanbeToggleWeapon
  (return (!= (Variables|Default|GetWeaponId) 0)))

(fn GetAttack
  (return (Math|Boolean|ANDBoolean (not (Variables|Default|GetIsAttacking)) (CallFunction|GetIsArmed) (Utilities|Enum|Equal(Enum) (Variables|Default|GetEquipState) "NewEnumerator0") (Pawn|Components|CharacterMovement|IsWalking (Variables|Character|GetCharacterMovement)))))

(fn SwordDamageTrace
  (bind _handweapon (Variables|Default|GetHandWeapon))
  (Utilities|IsValid _handweapon
    (:Is%20Valid
      (bind (_outhits _returnvalue) (Collision|MultiSphereTraceByChannel (Transformation|GetSocketLocation _handweapon "SwordDamageBeginSocket") (Transformation|GetSocketLocation _handweapon "SwordDamageEndSocket") 15.0 "TraceTypeQuery3" false 0 "ForDuration"))
      (bind _array_element (Utilities|Array|ForEachLoopwithBreak _outhits)
        (:LoopBody
          (Utilities|Array|AddUnique (LocalVariables|GetDamager) (.HitActor (Collision|BreakHitResult _array_element)))
          (return (LocalVariables|GetDamager) _returnvalue))
        (:Completed
          (return 0 false))))
    (:Is%20Not%20Valid
      (return 0 false))))

(fn BodyFootrDamageTrace
  (bind _mesh (Variables|Character|GetMesh))
  (Utilities|IsValid _mesh
    (:Is%20Valid
      (bind (_outhits _returnvalue) (Collision|MultiSphereTraceByChannel (Transformation|GetSocketLocation _mesh "DamageFootrStartSocket") (Transformation|GetSocketLocation _mesh "DamageFootrEndSocket") 15.0 "TraceTypeQuery3" false 0 "None"))
      (bind _array_element (Utilities|Array|ForEachLoopwithBreak _outhits)
        (:LoopBody
          (Utilities|Array|AddUnique (LocalVariables|GetDamager) (.HitActor (Collision|BreakHitResult _array_element)))
          (return (LocalVariables|GetDamager) _returnvalue))
        (:Completed
          (return 0 false))))
    (:Is%20Not%20Valid
      (return 0 false))))

(fn BodyFootlDamageTrace
  (bind _mesh (Variables|Character|GetMesh))
  (Utilities|IsValid _mesh
    (:Is%20Valid
      (bind (_outhits _returnvalue) (Collision|MultiSphereTraceByChannel (Transformation|GetSocketLocation _mesh "DamageFootlStartSocket") (Transformation|GetSocketLocation _mesh "DamageFootlEndSocket") 15.0 "TraceTypeQuery3" false 0 "None"))
      (bind _array_element (Utilities|Array|ForEachLoopwithBreak _outhits)
        (:LoopBody
          (Utilities|Array|AddUnique (LocalVariables|GetDamager) (.HitActor (Collision|BreakHitResult _array_element)))
          (return (LocalVariables|GetDamager) _returnvalue))
        (:Completed
          (return 0 false))))
    (:Is%20Not%20Valid
      (return 0 false))))

(fn CanTakeDamage
  (return (and (not (Variables|Default|GetIsDamaging)) (not (Variables|Default|GetIsRoll)))))

(fn CanRoll
  (return (Math|Boolean|ANDBoolean (Utilities|Enum|Equal(Enum) (Variables|Default|GetEquipState) "NewEnumerator0") (not (Variables|Default|GetIsAttacking)) (not (Variables|Default|GetIsDamaging)) (not (Variables|Default|GetIsRoll)) (CallFunction|GetIsArmed))))

(fn GetInputValue
  (return (Math|Trig|RadiansToDegrees (Class|KismetMathLibrary|VectorHeadingAngle (Math|Vector|Normalize (Math|Vector|MakeVector (Input|AxisValues|GetMoveForward) (Input|AxisValues|GetMoveRight) 0.0))))))

(fn GetRollSection
  (Utilities|FlowControl|Sequence
    (:then_0
      (if (and (< (Math|Float|Absolute(Float) (Default|GetInputValue (Variables|Default|GetAs%20PC%20BP))) (Math|Float|MakeLiteralFloat 45.0)) (>= (Math|Float|Absolute(Float) (Default|GetInputValue (Variables|Default|GetAs%20PC%20BP))) (Math|Float|MakeLiteralFloat 0.0)))
        (LocalVariables|SetSectionName "F")))
    (:then_1
      (if (and (>= (Default|GetInputValue (Variables|Default|GetAs%20PC%20BP)) (Math|Float|MakeLiteralFloat 45.0)) (< (Default|GetInputValue (Variables|Default|GetAs%20PC%20BP)) (Math|Float|MakeLiteralFloat 135.0)))
        (LocalVariables|SetSectionName "R")))
    (:then_2
      (if (and (<= (Default|GetInputValue (Variables|Default|GetAs%20PC%20BP)) (Math|Float|MakeLiteralFloat -45.0)) (> (Default|GetInputValue (Variables|Default|GetAs%20PC%20BP)) (Math|Float|MakeLiteralFloat -135.0)))
        (LocalVariables|SetSectionName "L")))
    (:then_3
      (if (and (>= (Math|Float|Absolute(Float) (Default|GetInputValue (Variables|Default|GetAs%20PC%20BP))) (Math|Float|MakeLiteralFloat 135.0)) (<= (Math|Float|Absolute(Float) (Default|GetInputValue (Variables|Default|GetAs%20PC%20BP))) (Math|Float|MakeLiteralFloat 1.8e+02)))
        (LocalVariables|SetSectionName "B")))
    (:then_4
      (return (LocalVariables|GetSectionName)))))

(fn GetSection
  (return (Utilities|Array|Get(acopy) (Variables|Default|GetAttackComboSections) (Variables|Default|GetCurrentAttackCombo))))

(fn SetCurrentAttackCombo
  (params (InCombo :type Integer))
  (Variables|Default|SetCurrentAttackCombo InCombo)
  (return))

(fn SetIsAttacking
  (params (InIsAttacking :type Boolean))
  (Variables|Default|SetIsAttacking InIsAttacking)
  (return))