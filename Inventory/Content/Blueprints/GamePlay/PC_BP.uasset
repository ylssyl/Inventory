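; Player controller that drives the player's BP_Character, turning input into movement, jumping and a walk-speed toggle on the Spring action.
; Movement follows the camera's forward and right vectors, and jump velocity is copied from the current max walk speed, so the toggle also changes jump height.
; ToggleMouseFunc switches cursor and input mode when the bag opens or closes, and GetInputValue returns the movement input's heading in degrees.
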(event EventBeginPlay
  (bind _ascharacter_bp (Utilities|Casting|CastToBP_Character (Game|Player|GetPlayerPawn 0)))
  (Variables|Default|SetAs%20Character%20BP _ascharacter_bp))

(event EventTick
  (params (DeltaSeconds :type Float%20%28single-precision%29)))

(event EventToggleMouseFunc
  (params (InIsBagOpened :type Boolean))
  (bind _self self)
  (if InIsBagOpened
    (Input|SetInputModeGameandUI _self 0 "LockAlways" true)
    (Variables|Default|SetbShowMouseCursor true)
    (else
      (Input|SetInputModeGameOnly _self)
      (Variables|Default|SetbShowMouseCursor false))))

(event Input|ActionEvents|InputActionJump
  (params (Key :type Key%20Structure))
  (bind _as_character_bp (Variables|Default|GetAs%20Character%20BP))
  (bind _as_character_bp_2 (Variables|Default|GetAs%20Character%20BP))
  (bind _charactermovement (Variables|/Script/Engine.Character|GetCharacterMovement _as_character_bp_2))
  (bind _maxwalkspeed (Variables|/Script/Engine.CharacterMovementComponent|GetMaxWalkSpeed _charactermovement))
  (:Pressed
    (Variables|/Script/Engine.CharacterMovementComponent|SetJumpZVelocity _charactermovement _maxwalkspeed)
    (Character|Jump _as_character_bp))
  (:Released
    (Variables|/Script/Engine.CharacterMovementComponent|SetJumpZVelocity _charactermovement _maxwalkspeed)
    (Character|StopJumping _as_character_bp)))

(event Input|ActionEvents|InputActionSpring
  (params (Key :type Key%20Structure))
  (bind _as_character_bp (Variables|Default|GetAs%20Character%20BP))
  (bind _charactermovement (Variables|/Script/Engine.Character|GetCharacterMovement _as_character_bp))
  (:Pressed
    (Utilities|FlowControl|FlipFlop
      (:A
        (Variables|/Script/Engine.CharacterMovementComponent|SetMaxWalkSpeed _charactermovement 6e+02))
      (:B
        (Variables|/Script/Engine.CharacterMovementComponent|SetMaxWalkSpeed _charactermovement 4.5e+02)))))

(event Input|AxisEvents|InputAxisMoveForward
  (params (AxisValue :type Float%20%28single-precision%29))
  (Pawn|Input|AddMovementInput (Game|Player|GetPlayerPawn 0) (Math|Vector|GetForwardVector (Camera|GetCameraRotation (Game|GetPlayerCameraManager 0))) AxisValue false))

(event Input|AxisEvents|InputAxisMoveRight
  (params (AxisValue :type Float%20%28single-precision%29))
  (Pawn|Input|AddMovementInput (Game|Player|GetPlayerPawn 0) (Math|Vector|GetRightVector (Camera|GetCameraRotation (Game|GetPlayerCameraManager 0))) AxisValue false))

(fn ConstructionScript)

(fn GetInputValue
  (return (Math|Trig|RadiansToDegrees (Class|KismetMathLibrary|VectorHeadingAngle (Math|Vector|Normalize (Math|Vector|MakeVector (Input|AxisValues|GetMoveForward) (Input|AxisValues|GetMoveRight) 0.0))))))