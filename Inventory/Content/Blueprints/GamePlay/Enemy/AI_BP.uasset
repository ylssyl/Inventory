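; AI_BP is an enemy AI controller that runs the AI_BT behavior tree and feeds its AI_BB blackboard.
; On BeginPlay it starts the tree and records the controlled pawn's location as SpawnLocation.
; AI Perception sight updates set PerceptionTarget and clear SuspicionLocation when a target is seen.
; When sight is lost, they clear the target and store the stimulus location as SuspicionLocation.
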(event OnTargetPerceptionUpdated(AIPerception)
  (params (Actor :type Actor%20Object%20Reference) (Stimulus :type AI%20Stimulus%20Structure))
  (bind (_age _expirationage _strength _stimuluslocation _receiverlocation _tag _bsuccessfullysensed) (Utilities|Struct|BreakAIStimulus Stimulus))
  (bind _returnvalue (Class|AIPerceptionSystem|GetSenseClassforStimulus Stimulus))
  (if (== _returnvalue "/Script/AIModule.AISense_Sight")
    (if _bsuccessfullysensed
      (AI|Components|Blackboard|SetValueasObject (AI|GetBlackboard self) (Utilities|Name|MakeLiteralName "PerceptionTarget") Actor)
      (AI|Components|Blackboard|ClearValue (AI|GetBlackboard self) (Utilities|Name|MakeLiteralName "SuspicionLocation"))
      (else
        (AI|Components|Blackboard|ClearValue (AI|GetBlackboard self) (Utilities|Name|MakeLiteralName "PerceptionTarget"))
        (AI|Components|Blackboard|SetValueasVector (AI|GetBlackboard self) (Utilities|Name|MakeLiteralName "SuspicionLocation") _stimuluslocation)))))

(event EventBeginPlay
  ;[1 1 1] 逻辑
  (AI|RunBehaviorTree "/Game/Blueprints/GamePlay/Enemy/AI_BT.AI_BT")
  ;[1 1 1] 记忆
  (Class|AIController|UseBlackboard "/Game/Blueprints/GamePlay/Enemy/AI_BB.AI_BB")
  (CallFunction|SetSpawnLocation))

(event EventTick
  (params (DeltaSeconds :type Float%20%28single-precision%29)))

(fn ConstructionScript)

(fn SetSpawnLocation
  (AI|Components|Blackboard|SetValueasVector (AI|GetBlackboard self) (Utilities|Name|MakeLiteralName "SpawnLocation") (Transformation|GetActorLocation (Pawn|GetControlledPawn))))