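; Sword-fighting enemy character with weapon equip, combo attacks, directional rolls, blocking, health widget display and timed ragdoll death.
; Try events check state guards before playing montages or setting flags, while begin/tick/end events handle rotation, curve-driven roll movement and combo index.
; Attack ticks sphere-trace between sword sockets to apply damage; received hits trigger GA_Damage through the Ability System unless blocking.
; Movement, view and input-style trigger chains are disconnected.
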(event EventDie
  (CallFunction|EnableRagDoll))

(event EventOnHealthChanged
  (params (Health :type Float%20%28single-precision%29) (MaxHealth :type Float%20%28single-precision%29))
  (Class|BPIShowAttribute|ShowHealth(Message) (UserInterface|GetUserWidgetObject (Variables|Default|GetWidget)) Health MaxHealth))

(event Input|ActionEvents|InputActionSpring
  (params (Key :type Key%20Structure)))

(event Input|ActionEvents|InputActionJump
  (params (Key :type Key%20Structure)))

(event Custom|OnToggleWeapon
  (params (IsEquip :type Boolean))
  (bind _charactermovement (Variables|Character|GetCharacterMovement))
  (Utilities|FlowControl|Sequence
    (:then_0
      (bind _output_get (Variables|/Script/Engine.CharacterMovementComponent|SetbUseControllerDesiredRotation _charactermovement IsEquip))
      (Variables|/Script/Engine.CharacterMovementComponent|SetbOrientRotationToMovement _charactermovement (not _output_get))
      (Variables|/Script/Engine.CharacterMovementComponent|SetMaxWalkSpeed (Variables|Character|GetCharacterMovement) (Math|Float|SelectFloat 4e+02 6e+02 IsEquip))
      (Variables|Default|SetCurrentAttackComb 0))
    (:then_1
      (Transformation|AttachComponentToComponent (Variables|Default|GetSword) (Variables|Character|GetMesh) (select IsEquip "Socket_Weapon" "Socket_WeaponSpine") "SnapToTarget" "SnapToTarget" "SnapToTarget" true))
    (:then_2
      (if IsEquip
        (Variables|Default|SetHandWeapon (Variables|Default|GetSword))
        (else
          (Variables|Default|SetHandWeapon 0))))))

(event Custom|TryToggleWeapon
  (Utilities|FlowControl|Sequence
    (:then_0
      (if (CallFunction|GetEquip)
        (Animation|Montage|PlayMontage (Variables|Character|GetMesh) "/Game/Blueprints/GamePlay/Enemy/Character/Animation/Equipment/Equipment_AM.Equipment_AM" 1.0 0.0 "Equip"
          (:OnBlendOut
            _)
          (:OnInterrupted
            _))
        (Variables|Default|SetEquipState "NewEnumerator0")))
    (:then_1
      (if (CallFunction|GetUnEquip)
        (Animation|Montage|PlayMontage (Variables|Character|GetMesh) "/Game/Blueprints/GamePlay/Enemy/Character/Animation/Equipment/Equipment_AM.Equipment_AM" 1.0 0.0 "UnEquip"
          (:OnBlendOut
            _)
          (:OnInterrupted
            _))
        (Variables|Default|SetEquipState "NewEnumerator0")))))

(event Custom|TryRoll
  (if (CallFunction|CanRoll)
    (Animation|Montage|PlayMontage (Variables|Character|GetMesh) "/Game/Blueprints/GamePlay/Enemy/Character/Animation/Roll/Roll_AM.Roll_AM" 1.0 0.0 (CallFunction|GetRollSection)
      (:then
        (Variables|Default|SetIsRolling true))
      (:OnInterrupted
        (CallFunction|OnEndRoll)))))

(event Custom|OnEndRoll
  (bind _charactermovement (Variables|Character|GetCharacterMovement))
  (Variables|Default|SetbCanBeDamaged true)
  (Variables|/Script/Engine.CharacterMovementComponent|SetbUseControllerDesiredRotation _charactermovement true)
  (Variables|/Script/Engine.CharacterMovementComponent|SetbOrientRotationToMovement _charactermovement false))

(event Custom|OnBeginRoll
  (bind _charactermovement (Variables|Character|GetCharacterMovement))
  (Variables|Default|SetbCanBeDamaged false)
  (Variables|/Script/Engine.CharacterMovementComponent|SetbUseControllerDesiredRotation _charactermovement false)
  (Variables|/Script/Engine.CharacterMovementComponent|SetbOrientRotationToMovement _charactermovement true)
  (Transformation|AddActorLocalRotation (Math|Rotator|MakeRotator 0.0 0.0 0.0) false false))

(event Custom|OnRollTick
  (params (DeltaTime :type Float%20%28single-precision%29))
  (bind _mesh (Variables|Character|GetMesh))
  (bind _returnvalue (Components|SkeletalMesh|GetAnimInstance _mesh))
  (Transformation|AddActorLocalOffset (* (* (Math|Vector|MakeVector (Animation|Curves|GetCurveValue _returnvalue "RollOffsetY") (* (Animation|Curves|GetCurveValue _returnvalue "RollOffsetX") -1.0) 0.0) (* (Math|Float|MakeLiteralFloat 3e+01) DeltaTime)) 2.0) true false))

(event Custom|OnAttack
  (params (DamageSection :type Name) (AttackDir :type Vector)))

(event Custom|TryAttack
  (if (CallFunction|GetAttack)
    (Animation|Montage|PlayMontage (Variables|Character|GetMesh) "/Game/Blueprints/GamePlay/Enemy/Character/Animation/Attack/Attack/Attack_AM.Attack_AM" 1.0 0.0 (Utilities|Array|Get(acopy) (Variables|Default|GetAttackCombSections) (Variables|Default|GetCurrentAttackComb))
      (:OnCompleted
        (Variables|Default|SetCurrentAttackComb 0))
      (:OnInterrupted
        (Variables|Default|SetIsAttacking false)))))

(event Custom|OnBeginAttack
  (Variables|Default|SetCurrentAttackComb (Math|Integer|%(Integer) (+ (Variables|Default|GetCurrentAttackComb) 1) (Utilities|Array|Length (Variables|Default|GetAttackCombSections)))))

(event Custom|OnAttackTick
  (params (DamageSection :type Name) (AttackLocation :type Vector))
  (bind (_damagerarray _successed) (CallFunction|DamageTest))
  (Variables|Default|SetDamageSection DamageSection)
  (Variables|Default|SetAttackLocation AttackLocation)
  (if _successed
    (for _array_element _damagerarray
      (Game|Damage|ApplyDamage _array_element 2e+01 (Pawn|GetController) self))))

(event Custom|OnEndAttack)

(event Custom|TryTakeDamage
  (params (DanageSection :type Name) (AttackLocation :type Vector) (Attator :type Object%20Object%20Reference))
  (if (CallFunction|CanTakeDamage)
    (Variables|Default|SetAttackerLocation AttackLocation)
    (if (not (Variables|Default|GetIsBlocking))
      (Abilities|TryActivateAbilitybyClass (Variables|Default|GetAbilitySystemComponent) "/Game/Blueprints/GameplayAbility/GA_Damage.GA_Damage_C" true))))

(event Custom|OnEndDamage
  (Animation|StopAnimMontage "/Game/Blueprints/GamePlay/Enemy/Character/Animation/Attack/Damage/Damage_AM.Damage_AM"))

(event Custom|OnBeginDamage)

(event Custom|OnDamageTick
  (params (DeltaTime :type Float%20%28single-precision%29))
  (CallFunction|TurnRotation))

(event Game|Damage|EventAnyDamage
  (params (Damage :type Float%20%28single-precision%29) (DamageType :type Damage%20Type%20Object%20Reference) (InstigatedBy :type Controller%20Object%20Reference) (DamageCauser :type Actor%20Object%20Reference))
  (bind (_danagesection _attackrlocation) (CallFunction|GetAttackerSection DamageCauser))
  (CallFunction|TryTakeDamage _danagesection _attackrlocation DamageCauser))

(event Custom|TryBlocking
  (if (CallFunction|CanBlocking)
    (Variables|Default|SetIsBlocking true)
    (Variables|/Script/Engine.CharacterMovementComponent|SetMaxWalkSpeed (Variables|Character|GetCharacterMovement) 2e+02)))

(event Custom|CancelBlocking
  (Variables|Default|SetIsBlocking false)
  (Variables|/Script/Engine.CharacterMovementComponent|SetMaxWalkSpeed (Variables|Character|GetCharacterMovement) 4e+02))

(event Custom|EnableRagDoll
  (Variables|Default|SetIsRagdoll true)
  (Physics|SetSimulatePhysics (Variables|Character|GetMesh) true)
  (Collision|SetCollisionEnabled (Variables|Character|GetMesh) "PhysicsOnly")
  (Collision|SetCollisionEnabled (Variables|Default|GetCapsuleComponent) "NoCollision")
  (Utilities|FlowControl|Delay 5.0)
  (Actor|DestroyActor))

(event Custom|DisableRagdoll
  (Variables|Default|SetIsRagdoll false))

(fn ConstructionScript)

(fn GetCameraRotation
  (return (Camera|GetCameraRotation (Game|GetPlayerCameraManager 0))))

(fn GetIsArmed
  (return (and (Utilities|IsValid (Variables|Default|GetHandWeapon)) (not (Variables|Default|GetIsRagdoll)))))

(fn GetEquip
  (return (and (or (Utilities|Enum|Equal(Enum) (Variables|Default|GetEquipState) "NewEnumerator0") (Utilities|Enum|Equal(Enum) (Variables|Default|GetEquipState) "NewEnumerator2")) (not (CallFunction|GetIsArmed)))))

(fn GetUnEquip
  (return (Math|Boolean|ANDBoolean (or (Utilities|Enum|Equal(Enum) (Variables|Default|GetEquipState) "NewEnumerator1") (Utilities|Enum|Equal(Enum) (Variables|Default|GetEquipState) "NewEnumerator0")) (CallFunction|GetIsArmed) (not (Variables|Default|GetIsAttacking)))))

(fn GetAttack
  (return (Math|Boolean|ANDBoolean (not (Variables|Default|GetIsAttacking)) (CallFunction|GetIsArmed) (Utilities|Enum|Equal(Enum) (Variables|Default|GetEquipState) "NewEnumerator0") (Pawn|Components|CharacterMovement|IsWalking (Variables|Character|GetCharacterMovement)))))

(fn DamageTest
  (bind _handweapon (Variables|Default|GetHandWeapon))
  (Utilities|IsValid _handweapon
    (:Is%20Valid
      (bind (_outhits _returnvalue) (Collision|MultiSphereTraceByChannel (Transformation|GetSocketLocation _handweapon "DamageTestBeginSocket") (Transformation|GetSocketLocation _handweapon "DamageTestEndSocket") 15.0 "TraceTypeQuery3" false 0 "None"))
      (bind _array_element (Utilities|Array|ForEachLoopwithBreak _outhits)
        (:LoopBody
          (Utilities|Array|AddUnique (LocalVariables|GetDamagers) (.HitActor (Collision|BreakHitResult _array_element)))
          (return (LocalVariables|GetDamagers) _returnvalue))
        (:Completed
          (return 0 false))))
    (:Is%20Not%20Valid
      (return 0 false))))

(fn CanTakeDamage
  (return (and (not (Variables|Default|GetIsDamaging)) (not (Variables|Default|GetIsRagdoll)))))

(fn CanBlocking
  (return (Math|Boolean|ANDBoolean (not (Variables|Default|GetIsBlocking)) (CallFunction|GetIsArmed) (not (Variables|Default|GetIsAttacking)) (not (Variables|Default|GetIsDamaging)) (Utilities|Enum|Equal(Enum) (Variables|Default|GetEquipState) "NewEnumerator0"))))

(fn BlockTest
  (bind _returnvalue (Transformation|GetActorLocation))
  (if (Math|Boolean|ANDBoolean (Variables|Default|GetIsBlocking) (CallFunction|GetIsArmed) (not (Variables|Default|GetIsAttacking)) (not (Variables|Default|GetIsDamaging)) (Utilities|Enum|Equal(Enum) (Variables|Default|GetEquipState) "NewEnumerator0"))
    (bind (_outhits _returnvalue_2) (Collision|MultiSphereTraceByChannel _returnvalue (+ _returnvalue "0, 0,1.000000") 2.5e+02 "TraceTypeQuery3" false 0 "None"))
    (bind _array_element (Utilities|Array|ForEachLoopwithBreak _outhits)
      (:LoopBody
        (Utilities|Array|AddUnique (LocalVariables|GetBlocker) (.HitActor (Collision|BreakHitResult _array_element)))
        (return (LocalVariables|GetBlocker) _returnvalue_2)))
    (else
      (return 0 false))))

(fn TurnRotation
  (Transformation|SetActorRotation (Math|Rotator|MakeRotator 0.0 0.0 (Math|Float|Lerp (.yaw (Math|Conversions|RotationFromXVector (Math|Vector|GetUnitDirection(Vector) (Transformation|GetActorLocation) (Variables|Default|GetAttackerLocation)))) 0.0 0.2))))

(fn CanRoll
  (return (Math|Boolean|ANDBoolean (CallFunction|GetIsArmed) (Utilities|Enum|Equal(Enum) (Variables|Default|GetEquipState) "NewEnumerator0") (not (Variables|Default|GetIsAttacking)) (not (Variables|Default|GetIsDamaging)) (not (Variables|Default|GetIsRolling)))))

(fn CanJumpInternal
  (return (Math|Boolean|ANDBoolean (not (Utilities|IsValid (Variables|Default|GetHandWeapon))) (Utilities|Enum|Equal(Enum) (Variables|Default|GetEquipState) "NewEnumerator0") (not (Variables|Default|GetIsAttacking)) (not (Variables|Default|GetIsDamaging)))))

(fn GetRollSection
  (Utilities|FlowControl|Sequence
    (:then_0
      (if (and (< (Math|Float|Absolute(Float) (CallFunction|GetInputValue)) (Math|Float|MakeLiteralFloat 22.5)) (>= (Math|Float|Absolute(Float) (CallFunction|GetInputValue)) (Math|Float|MakeLiteralFloat 0.0)))
        (LocalVariables|SetSectionName "F")))
    (:then_1
      (if (and (>= (CallFunction|GetInputValue) (Math|Float|MakeLiteralFloat 22.5)) (< (CallFunction|GetInputValue) (Math|Float|MakeLiteralFloat 67.5)))
        (LocalVariables|SetSectionName "FR")))
    (:then_2
      (if (and (>= (CallFunction|GetInputValue) (Math|Float|MakeLiteralFloat 67.5)) (< (CallFunction|GetInputValue) (Math|Float|MakeLiteralFloat 112.5)))
        (LocalVariables|SetSectionName "R")))
    (:then_3
      (if (and (>= (CallFunction|GetInputValue) (Math|Float|MakeLiteralFloat 112.5)) (< (CallFunction|GetInputValue) (Math|Float|MakeLiteralFloat 157.5)))
        (LocalVariables|SetSectionName "BR")))
    (:then_4
      (if (and (<= (CallFunction|GetInputValue) (Math|Float|MakeLiteralFloat -22.5)) (> (CallFunction|GetInputValue) (Math|Float|MakeLiteralFloat -67.5)))
        (LocalVariables|SetSectionName "FL")))
    (:then_5
      (if (and (<= (CallFunction|GetInputValue) (Math|Float|MakeLiteralFloat -67.5)) (> (CallFunction|GetInputValue) (Math|Float|MakeLiteralFloat -112.5)))
        (LocalVariables|SetSectionName "L")))
    (:then_6
      (if (and (<= (CallFunction|GetInputValue) (Math|Float|MakeLiteralFloat -112.5)) (> (CallFunction|GetInputValue) (Math|Float|MakeLiteralFloat -157.5)))
        (LocalVariables|SetSectionName "BL")))
    (:then_7
      (if (and (>= (Math|Float|Absolute(Float) (CallFunction|GetInputValue)) (Math|Float|MakeLiteralFloat 157.5)) (<= (Math|Float|Absolute(Float) (CallFunction|GetInputValue)) (Math|Float|MakeLiteralFloat 1.8e+02)))
        (LocalVariables|SetSectionName "B")))
    (:then_8
      (return (LocalVariables|GetSectionName)))))

(fn GetInputValue
  (return (Math|Trig|RadiansToDegrees (Class|KismetMathLibrary|VectorHeadingAngle (Math|Vector|Normalize (Math|Vector|MakeVector (Input|AxisValues|GetMoveForward) (Input|AxisValues|GetMoveRight) 0.0))))))

(fn GetAttackerSection
  (params (AttackActor :type Actor%20Object%20Reference))
  (LocalVariables|SetYaw (CallFunction|GetAttackYaw AttackActor))
  (Utilities|FlowControl|Sequence
    (:then_0
      (if (and (< (Math|Float|Absolute(Float) (LocalVariables|GetYaw)) (Math|Float|MakeLiteralFloat 45.0)) (>= (Math|Float|Absolute(Float) (LocalVariables|GetYaw)) (Math|Float|MakeLiteralFloat 0.0)))
        (LocalVariables|SetSectionName "1")))
    (:then_1
      (if (and (>= 0.0 (Math|Float|MakeLiteralFloat 45.0)) (< (LocalVariables|GetYaw) (Math|Float|MakeLiteralFloat 135.0)))
        (LocalVariables|SetSectionName "3")))
    (:then_2
      (if (and (<= (LocalVariables|GetYaw) (Math|Float|MakeLiteralFloat -45.0)) (> (LocalVariables|GetYaw) (Math|Float|MakeLiteralFloat -135.0)))
        (LocalVariables|SetSectionName "2")))
    (:then_3
      (if (and (>= (Math|Float|Absolute(Float) (LocalVariables|GetYaw)) (Math|Float|MakeLiteralFloat 135.0)) (<= (Math|Float|Absolute(Float) (LocalVariables|GetYaw)) (Math|Float|MakeLiteralFloat 1.8e+02)))
        (LocalVariables|SetSectionName "0")))
    (:then_4
      (return (LocalVariables|GetSectionName) (Transformation|GetActorLocation AttackActor)))))

(fn GetAttackYaw
  (params (InputActor :type Actor%20Object%20Reference))
  (return (.yaw (Math|Conversions|RotationFromXVector (Math|Vector|GetUnitDirection(Vector) (Transformation|GetActorLocation self) (Transformation|GetActorLocation InputActor))))))