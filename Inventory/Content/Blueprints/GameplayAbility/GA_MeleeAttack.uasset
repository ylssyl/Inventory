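; Gameplay Ability for a melee attack that plays a montage and damages targets reported during it.
; On activation it commits, then plays AM_AttackAnim from the section the owning actor returns through a message call.
; While active, it waits for Skill.melee.dealDamage events and applies GE_MeleeDamage to each payload target.
; Completion passes CurrentAttackCombo to the owner, interruption passes IsAttacking, and every montage exit, including blend-out, ends the ability.
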(event Ability|EventActivateAbility
  (bind _returnvalue (Ability|GetOwningActorfromActorInfo))
  (Ability|CommitAbility)
  (bind _outsection (Class|BPIMeleeAttack|GetSection(Message) _returnvalue))
  (|PlayMontageandWaitProxy "None" "/Game/Blueprints/Animation/Attack/AM_AttackAnim.AM_AttackAnim" 1.0 _outsection true 1.0 0.0
    (:then
      (bind _payload (Ability|Tasks|WaitGameplayEvent "(TagName=\"skill.melee.dealDamage\")" 0)
        (:EventReceived
          (GameplayEffects|ApplyGameplayEffectToTarget (Ability|TargetData|AbilityTargetDatafromActor (.Target (Utilities|Struct|BreakGameplayEventData _payload))) "/Game/Blueprints/GameplayAbility/GE_MeleeDamage.GE_MeleeDamage_C" 1 1))))
    (:OnCompleted
      (Class|BPIMeleeAttack|SetCurrentAttackCombo(Message) _returnvalue (Variables|Default|GetCurrentAttackCombo))
      (Ability|EndAbility :!label _label))
    (:OnBlendOut
      (goto _label))
    (:OnInterrupted
      (Class|BPIMeleeAttack|SetIsAttacking(Message) _returnvalue (Variables|Default|GetIsAttacking))
      (goto _label))
    (:OnCancelled
      (goto _label))))

(event Ability|EventOnEndAbility
  (params (bWasCancelled :type Boolean)))

(fn GetCurrentAttackCombo
  (return (Variables|Default|GetCurrentAttackCombo)))

(fn GetIsAttacking
  (return (Variables|Default|GetIsAttacking)))

(fn GetSection
  (return "None"))